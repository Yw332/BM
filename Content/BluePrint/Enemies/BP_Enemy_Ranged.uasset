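; Ranged enemy Blueprint that fires arrows at its AI controller's attack target and supplies its movement speeds and ideal combat ranges.
; Attack plays a montage whose notify picks an aim point in a spread cone, replaced by the impact point if a weapon-to-target trace hits.
; It spawns BP_Weapon_Arrow from a mesh socket toward that point and starts a timed recovery.
; Montage completion or interruption calls OnAttackEnd.
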(event `/Game/BluePrint/Enemies/AI/BPI_Enemy_AI.Attack`
  (bind _returnvalue (`self.K2_GetActorLocation` (`self.WeaponActor`)))
  (bind _notifyname (`|PlayMontage` (`self.Mesh`) "/Game/Asset/Animation/Enemy/Ranged/AM_Lang08_Attack10.AM_Lang08_Attack10")
    (:`OnCompleted`
      (`self.OnAttackEnd` :!label _label))
    (:`OnInterrupted`
      (goto _label))
    (:`OnNotifyBegin`
      (switch `name` _notifyname
        (:`fire`
          (bind _asaic_enemy_base (cast `/Game/BluePrint/Enemies/AI/AIC_Enemy_Base` (`AIBlueprintHelperLibrary.GetAIController` self)))
          (bind _attack_target (`/Game/BluePrint/Enemies/AI/AIC_Enemy_Base.Attack Target` _asaic_enemy_base)
            (:`then`
              (`|ExecutionSequence`
                (:`then_0`
                  (bind _returnvalue_2 (`self.K2_GetActorLocation` _attack_target))
                  (set `self.CrosshairWorldLocation` _returnvalue_2)
                  (set `self.ImpartPoint` (+ (`self.ArrowSpawnLocation`) (* (`KismetMathLibrary.RandomUnitVectorInEllipticalConeInDegrees` (`KismetMathLibrary.Normal` (- _returnvalue_2 _returnvalue)) (`self.SpreadAngleDeg`) (`self.SpreadAngleDegVertical`)) (`self.MaxFireDistance`)))))
                (:`then_1`
                  (bind _outhit (`KismetSystemLibrary.LineTraceSingle` _returnvalue (`self.CrosshairWorldLocation`) "TraceTypeQuery1" false (`|MakeArray` self :!type "Actor Object Reference")))
                  (bind (_bblockinghit _binitialoverlap _time _distance _location _impactpoint) (`GameplayStatics.BreakHitResult` _outhit))
                  (if _bblockinghit
                    (set `self.ImpartPoint` _impactpoint))
                  (set `self.ArrowSpawnLocation` (.location (`SceneComponent.GetSocketTransform` (`self.Mesh`) "Hit_Arrow_1" "RTS_World")))
                  (set `self.ArrowSpawnRotation` (`KismetMathLibrary.MakeRotFromX` (- (`self.ImpartPoint`) (`self.ArrowSpawnLocation`)))))
                (:`then_2`
                  (`|SpawnActorFromClass` "/Game/BluePrint/Enemies/Weapon/BP_Weapon_Arrow.BP_Weapon_Arrow_C" (`KismetMathLibrary.MakeTransform` (`self.ArrowSpawnLocation`) (`self.ArrowSpawnRotation`)) "AdjustIfPossibleButAlwaysSpawn" "MultiplyWithRoot" self self)
                  (set `self.bIsInRecovery` true)
                  (`KismetSystemLibrary.K2_SetTimerDelegate` (`|CreateDelegate` :!event `ClearRecovery`) (`self.RecoveryTime`)))))
            (:`else`)))))))

(event `self.ReceiveBeginPlay`
  (`parent.ReceiveBeginPlay`))

(event `ClearRecovery`
  (set `self.bIsInRecovery` false))

(fn `GetIdealRange`
  (returns (AttackRadius :type "Float (double-precision)") (DefendRadius :type "Float (double-precision)"))
  (return 1500.0 1800.0))

(fn `GetPatrolRoute`
  (returns (PatrolRoute :type "/Game/BluePrint/Enemies/AI/BP_PatrolRoute Object Reference"))
  (return null))

(fn `SetMovementSpeed`
  (params (Speed :type "/Game/BluePrint/Enemies/AI/Enums/E_AISpeed Enum" :default "NewEnumerator0"))
  (returns (SpeedValue :type "Float (double-precision)"))
  (bind _output_get (set `CharacterMovementComponent.MaxWalkSpeed` (select `/Game/BluePrint/Enemies/AI/Enums/E_AISpeed` Speed :`NewEnumerator1` 200.0 :`NewEnumerator2` 400.0 :!type "Float (single-precision)") (`self.CharacterMovement`)))
  (return _output_get))

(fn `UserConstructionScript`
  (`parent.UserConstructionScript`))