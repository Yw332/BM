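; Enemy arrow projectile that damages the player on contact and sticks to them.
; LaunchArrow adds a projectile movement component at runtime with the given velocity and zero gravity.
; When the Box overlaps the player, the owning BP_Enemy_Base deals fixed damage through DoDamageToActor.
; The arrow then stops its ProjectileMovement, attaches to the player keeping world transform, and disables Box collision; other actors are ignored.
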(event `LaunchArrow`
  (params (`速度` :type "Vector Structure"))
  (bind _returnvalue (`AddComponent|NODE_AddProjectileMovementComponent-0`))
  (bind _output_get (set `self.ProjectileMovementRef` _returnvalue))
  (set `MovementComponent.Velocity` `速度` _output_get)
  (set `ProjectileMovementComponent.ProjectileGravityScale` 0.0 _returnvalue))

(event `self.Box.OnComponentBeginOverlap`
  (params (OverlappedComponent :type "PrimitiveComponent Object Reference") (OtherActor :type "Actor Object Reference") (OtherComp :type "PrimitiveComponent Object Reference") (OtherBodyIndex :type Integer) (bFromSweep :type Boolean) (SweepResult :type "HitResult Structure (by ref)"))
  (bind _projectilemovement (`self.ProjectileMovement`))
  (if (!= OtherActor self)
    (bind _asbp_bmplayer_character (cast `/Game/BluePrint/Player/Character/BP_BMPlayerCharacter` OtherActor))
    (bind _asbp_enemy_base (cast `/Game/BluePrint/Enemies/BP_Enemy_Base` (`self.GetOwner`)))
    (`BMNPCCharacter.DoDamageToActor` _asbp_enemy_base _asbp_bmplayer_character 10.0)
    (`MovementComponent.StopMovementImmediately` _projectilemovement)
    (set `ProjectileMovementComponent.ProjectileGravityScale` 0.0 _projectilemovement)
    (`self.K2_AttachToActor` OtherActor "None" "KeepWorld" "KeepWorld" "KeepWorld")
    (`PrimitiveComponent.SetCollisionEnabled` (`self.Box`) "NoCollision")))

(fn `UserConstructionScript`)