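; Enemy sword weapon Blueprint that damages the player character on contact.
; When its Box component begins an overlap while CanCauseDamage is true, it casts the other actor to BP_BMPlayerCharacter and its owner to BP_Enemy_Base.
; The owning enemy then applies fixed damage through DoDamageToActor, and the flag clears to prevent repeat hits.
; Nothing in this Blueprint sets the flag back to true.
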(event `self.Box.OnComponentBeginOverlap`
  (params (OverlappedComponent :type "PrimitiveComponent Object Reference") (OtherActor :type "Actor Object Reference") (OtherComp :type "PrimitiveComponent Object Reference") (OtherBodyIndex :type Integer) (bFromSweep :type Boolean) (SweepResult :type "HitResult Structure (by ref)"))
  (if (`self.CanCauseDamage`)
    (bind _asbp_bmplayer_character (cast `/Game/BluePrint/Player/Character/BP_BMPlayerCharacter` OtherActor))
    (bind _asbp_enemy_base (cast `/Game/BluePrint/Enemies/BP_Enemy_Base` (`self.GetOwner`)))
    (`BMNPCCharacter.DoDamageToActor` _asbp_enemy_base _asbp_bmplayer_character 10.0)
    (set `self.CanCauseDamage` false)))

(fn `UserConstructionScript`
  (`parent.UserConstructionScript`))