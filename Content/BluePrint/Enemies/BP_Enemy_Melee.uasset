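; Melee enemy Blueprint that supplies the montage-driven actions, movement speeds, patrol route and combat ranges for its AI.
; Attack entry, jump back and online idle play montages and signal their end on completion or interruption, with an attack-entry notify setting the sword-drawing flag.
; Hit reactions pause the Behavior Tree, play a montage by hit direction (front and back share one), then report completion after a delay; the reaction-end event resumes the tree.
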(event `self.ReceiveBeginPlay`
  (`parent.ReceiveBeginPlay`))

(event `/Game/BluePrint/Enemies/AI/BPI_Enemy_AI.EnterAttack`
  (bind _notifyname (`|PlayMontage` (`self.Mesh`) "/Game/Asset/Animation/Enemy/Melee/Lang05/AM_Lang05_EnterAttack_Montage.AM_Lang05_EnterAttack_Montage")
    (:`OnCompleted`
      (`self.OnEnterAttackEnd` :!label _label))
    (:`OnInterrupted`
      (goto _label))
    (:`OnNotifyBegin`
      (switch `name` _notifyname
        (:`DrawSword`
          (set `self.IsDrawingSword` true))))))

(event `/Game/BluePrint/Enemies/AI/BPI_Enemy_AI.JumpBack`
  (`|PlayMontage` (`self.Mesh`) "/Game/Asset/Animation/Enemy/Melee/Lang05/AM_GYCY_Lang_05_Online_Jump_B_01_Montage.AM_GYCY_Lang_05_Online_Jump_B_01_Montage"
    (:`OnCompleted`
      _)
    (:`OnInterrupted`
      _))
  (`self.OnJumpBackEnd`))

(event `self.OnHitReactBegin`
  (params (DamageCauser :type "Actor Object Reference"))
  (bind _mesh (`self.Mesh`))
  (`self.PauseBehaviorTree`)
  (switch `EBMHitDirection` (`self.ComputeHitDirection` DamageCauser)
    (:`Front`
      (`|PlayMontage` _mesh "/Game/Asset/Animation/Enemy/Melee/Lang05/AM_GYCY_Lang_05_Online_Hit_Fast_Torso_F_02_Montage.AM_GYCY_Lang_05_Online_Hit_Fast_Torso_F_02_Montage"
        (:`OnCompleted`
          _)
        (:`OnInterrupted`
          _)))
    (:`Back`
      (`|PlayMontage` _mesh "/Game/Asset/Animation/Enemy/Melee/Lang05/AM_GYCY_Lang_05_Online_Hit_Fast_Torso_F_02_Montage.AM_GYCY_Lang_05_Online_Hit_Fast_Torso_F_02_Montage"
        (:`OnCompleted`
          _)
        (:`OnInterrupted`
          _)))
    (:`Left`
      (`|PlayMontage` _mesh "/Game/Asset/Animation/Enemy/Melee/Lang05/AM_GYCY_Lang_05_Online_Hit_Fast_Torso_L_01_Montage.AM_GYCY_Lang_05_Online_Hit_Fast_Torso_L_01_Montage"
        (:`OnCompleted`
          _)
        (:`OnInterrupted`
          _)))
    (:`Right`
      (`|PlayMontage` _mesh "/Game/Asset/Animation/Enemy/Melee/Lang05/AM_GYCY_Lang_05_Online_Hit_Fast_Torso_R_01_Montage.AM_GYCY_Lang_05_Online_Hit_Fast_Torso_R_01_Montage"
        (:`OnCompleted`
          _)
        (:`OnInterrupted`
          _))))
  (`KismetSystemLibrary.Delay` 0.8)
  (`self.NotifyHitReactComplete`))

(event `self.OnHitReactEnd`
  (`self.ResumeBehaviorTree`))

(event `PlayOnlineIdle`
  (`|PlayMontage` (`self.Mesh`) "/Game/Asset/Animation/Enemy/Melee/Lang05/AM_Idle_Online.AM_Idle_Online"
    (:`OnCompleted`
      _)
    (:`OnInterrupted`
      _))
  (`self.OnPlayOnlineIdleEnd`))

(fn `GetIdealRange`
  (returns (AttackRadius :type "Float (double-precision)") (DefendRadius :type "Float (double-precision)"))
  (return 500.0 800.0))

(fn `GetPatrolRoute`
  (returns (PatrolRoute :type "/Game/BluePrint/Enemies/AI/BP_PatrolRoute Object Reference"))
  (return (`self.PatrolRoute`)))

(fn `SetMovementSpeed`
  (params (Speed :type "/Game/BluePrint/Enemies/AI/Enums/E_AISpeed Enum" :default "NewEnumerator0"))
  (returns (SpeedValue :type "Float (double-precision)"))
  (bind _output_get (set `CharacterMovementComponent.MaxWalkSpeed` (select `/Game/BluePrint/Enemies/AI/Enums/E_AISpeed` Speed :`NewEnumerator1` 90.0 :`NewEnumerator2` 400.0 :!type "Float (single-precision)") (`self.CharacterMovement`)))
  (return _output_get))

(fn `UserConstructionScript`
  (`parent.UserConstructionScript`))