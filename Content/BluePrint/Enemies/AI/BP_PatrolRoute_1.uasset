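; BP_PatrolRoute_1 is an enemy AI patrol route that supplies world-space waypoints from a spline.
; IncrementPatrolRoute1 steps PatrolIndex along the spline points, flipping Direction at the last and first points so the route runs back and forth.
; GetSplinePointAsWorldPosition returns the world location of the spline point at the current index.
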(event `IncrementPatrolRoute1`
  (bind _output_get (set `self.Patrol index` (+ (`self.Patrol index`) (`self.Direction`))))
  (if (== _output_get (- (`SplineComponent.GetNumberOfSplinePoints` (`self.PatrolRoute1`)) 1))
    (set `self.Direction` -1)
    (elif (== (`self.Patrol index`) 0)
      (set `self.Direction` 1))))

(fn `GetSplinePointAsWorldPosition`
  (returns (Location :type "Vector Structure"))
  (return (`SplineComponent.GetLocationAtSplinePoint` (`self.PatrolRoute1`) (`self.Patrol Index`) "World")))

(fn `UserConstructionScript`)