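; Elite enemy character that extends a parent enemy class with two montage-driven melee attacks and a hit reaction.
; Each attack enables damage on its BP_Weapon_Base weapon, then signals attack end when the montage completes or is interrupted.
; Hit reactions pause the behavior tree, play a montage, notify completion after a short delay, and resume the tree on react end.
; It also supplies walk speeds per movement state and ideal attack and defend ranges.
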(event `self.ReceiveBeginPlay`
  (`parent.ReceiveBeginPlay`))

(event `/Game/BluePrint/Enemies/AI/BPI_Enemy_AI.Attack`
  (bind _asbp_weapon_base (cast `/Game/BluePrint/Enemies/Weapon/BP_Weapon_Base` (`self.WeaponActor`)))
  (set `/Game/BluePrint/Enemies/Weapon/BP_Weapon_Base.CanCauseDamage` true _asbp_weapon_base)
  (`|PlayMontage` (`self.Mesh`) "/Game/Asset/Animation/Enemy/Elites/AM_HFM_Niu_01_Atk_Fast_01_Montage1.AM_HFM_Niu_01_Atk_Fast_01_Montage1"
    (:`OnCompleted`
      _)
    (:`OnInterrupted`
      _))
  (`self.OnAttackEnd`))

(event `/Game/BluePrint/Enemies/AI/BPI_Enemy_AI.Attack2`
  (bind _asbp_weapon_base (cast `/Game/BluePrint/Enemies/Weapon/BP_Weapon_Base` (`self.WeaponActor`)))
  (set `/Game/BluePrint/Enemies/Weapon/BP_Weapon_Base.CanCauseDamage` true _asbp_weapon_base)
  (`|PlayMontage` (`self.Mesh`) "/Game/Asset/Animation/Enemy/Elites/AM_NIU_Attack2.AM_NIU_Attack2"
    (:`OnCompleted`
      _)
    (:`OnInterrupted`
      _))
  (`self.OnAttackEnd`))

(event `self.OnHitReactBegin`
  (params (DamageCauser :type "Actor Object Reference"))
  (`self.PauseBehaviorTree`)
  (`|PlayMontage` (`self.Mesh`) "/Game/Asset/Animation/Enemy/Elites/AM_NIU_Behit_F.AM_NIU_Behit_F"
    (:`OnCompleted`
      _)
    (:`OnInterrupted`
      _))
  (`KismetSystemLibrary.Delay` 0.8)
  (`self.NotifyHitReactComplete`))

(event `self.OnHitReactEnd`
  (`self.ResumeBehaviorTree`))

(fn `GetIdealRange`
  (returns (AttackRadius :type "Float (double-precision)") (DefendRadius :type "Float (double-precision)"))
  (return 1300.0 1300.0))

(fn `SetMovementSpeed`
  (params (Speed :type "/Game/BluePrint/Enemies/AI/Enums/E_AISpeed Enum" :default "NewEnumerator0"))
  (returns (SpeedValue :type "Float (double-precision)"))
  (bind _output_get (set `CharacterMovementComponent.MaxWalkSpeed` (select `/Game/BluePrint/Enemies/AI/Enums/E_AISpeed` Speed :`NewEnumerator1` 200.0 :`NewEnumerator2` 400.0 :!type "Float (single-precision)") (`self.CharacterMovement`)))
  (return _output_get))

(fn `UserConstructionScript`
  (`parent.UserConstructionScript`))