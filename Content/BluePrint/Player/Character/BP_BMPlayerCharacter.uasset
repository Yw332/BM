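; Player character Blueprint that manages its overhead HP bar widget and offers debug slow-motion keys.
; On BeginPlay and Possessed it hides the widget for the locally controlled character, otherwise printing a debug string.
; Health change events push a normalized percent into the UI_EnemyHPBar widget.
; Debug subtract and add keys slow and restore global time dilation.
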(event Collision|EventActorBeginOverlap
  (params (OtherActor :type Actor%20Object%20Reference)))

(event EventTick
  (params (DeltaSeconds :type Float%20%28single-precision%29)))

(event EventEventHealthChanged
  (params (Value :type Float%20%28single-precision%29))
  (bind _asui_enemy_hpbar (Utilities|Casting|CastToUI_EnemyHPBar (UserInterface|GetWidget (Variables|Default|GetWidget))))
  (Default|SetPercent _asui_enemy_hpbar (/ Value 1e+02)))

(event EventPossessed
  (params (NewController :type Controller%20Object%20Reference))
  (bind _widget (Variables|Default|GetWidget))
  (bind _returnvalue (UserInterface|GetWidget _widget))
  (if (Pawn|IsLocallyControlled self)
    (Utilities|IsValid _returnvalue
      (:Is%20Valid
        (Widget|SetVisibility _returnvalue "Hidden")))
    (else
      (Development|PrintString "Hello" true true "(R=0.000000,G=0.660000,B=1.000000,A=1.000000)" 1e+01))))

(event EventBeginPlay
  (bind _widget (Variables|Default|GetWidget))
  (bind _returnvalue (UserInterface|GetWidget _widget))
  (if (Pawn|IsLocallyControlled self)
    (Utilities|IsValid _returnvalue
      (:Is%20Valid
        (Widget|SetVisibility _returnvalue "Hidden")))
    (else
      (Development|PrintString "Hello" true true "(R=0.000000,G=0.660000,B=1.000000,A=1.000000)" 1e+01))))

(event Input|KeyboardEvents|DebugKeySubtract
  (params (Key :type Key%20Structure :default "None") (ActionValue :type Input%20Action%20Value%20Structure))
  (:Pressed
    (Utilities|Time|SetGlobalTimeDilation 0.2)))

(event Input|KeyboardEvents|DebugKeyAdd
  (params (Key :type Key%20Structure :default "None") (ActionValue :type Input%20Action%20Value%20Structure))
  (:Pressed
    (Utilities|Time|SetGlobalTimeDilation 1.0)))

(fn ConstructionScript)